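; EmisiveSound is an actor that animates three components, Grande, Mediana and Pequeña, as growing pulses, apparently visualizing emitted sound.
; Shortly after BeginPlay, a Timeline track's value selects which component grows in turn, resetting another to small scale.
; Growth adds a fixed step per update, so it depends on frame rate, and debug strings print each stage.
; An unconnected Plane3 scaling branch never runs.
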(event `self.ReceiveBeginPlay`
  (`KismetSystemLibrary.Delay` 0.2)
  (bind (_direction _newtrack_0) (`Timeline|Timeline_0`)
    (:`Update`
      (if (>= _newtrack_0 0.1)
        (if (>= _newtrack_0 2.0)
          (`SceneComponent.SetWorldScale3D` (`self.Grande`) (0.1 0.1 0.1))
          (if (>= _newtrack_0 3.0)
            (`SceneComponent.SetWorldScale3D` (`self.Mediana`) (0.1 0.1 0.1))
            (`SceneComponent.SetWorldScale3D` (`self.Pequeña`) (+ (`KismetMathLibrary.Conv_DoubleToVector` 0.1) (`SceneComponent.K2_GetComponentScale` (`self.Pequeña`))))
            (`KismetSystemLibrary.PrintString` "peque")
            (else
              (`SceneComponent.SetWorldScale3D` (`self.Mediana`) (+ (`KismetMathLibrary.Conv_DoubleToVector` 0.1) (`SceneComponent.K2_GetComponentScale` (`self.Mediana`))))
              (`KismetSystemLibrary.PrintString` "mediano")))
          (else
            (`SceneComponent.SetWorldScale3D` (`self.Grande`) (+ (`KismetMathLibrary.Conv_DoubleToVector` 0.1) (`SceneComponent.K2_GetComponentScale` (`self.Grande`))))
            (`KismetSystemLibrary.PrintString` "grande")))
        (else
          (`SceneComponent.SetWorldScale3D` (`self.Pequeña`) (0.1 0.1 0.1)))))))

(fn `UserConstructionScript`)